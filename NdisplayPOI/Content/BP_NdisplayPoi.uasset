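; nDisplay point-of-interest marker that shows an image billboard at the end of a drawn leader line.
; Construction offsets the billboard from the last line point by a direction enum, scales it from editor settings and applies the image through a dynamic material.
; Tick uses paired DoOnce gates to hide it when GI_Nanjing's last index is non-zero, otherwise show it only if its tag matches the current level, redrawing lines while visible.
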(event EventBeginPlay
  (bind _asgi_nanjing (Utilities|Casting|CastToGI_Nanjing (Game|GetGameInstance)))
  (Variables|Default|SetGameInstance _asgi_nanjing))

(event EventTick
  (params (DeltaSeconds :type Float%20%28single-precision%29))
  (Utilities|FlowControl|Sequence
    (:then_0
      (if (Variables|/Game/Blueprints/GI_Nanjing.GI_Nanjing_C|GetbIsLastIndexNotZero (Variables|Default|GetGameInstance)) ; 判断最后一位是否不为0
        (Utilities|FlowControl|Sequence ; 最后一位若不为0则隐藏POI
          (:then_0
            (Utilities|FlowControl|DoOnce false :!label _label
              (:Completed
                (Development|SetHiddeninGame (Variables|Default|GetMaterialBiilboradComp) true false) ; 最后一位若不为0则隐藏POI
                (Class|NdisplayPoiActor|ClearAllNdisplayPoiLines) ; 清除所有线条
                (Variables|Default|SetbShouldDrawBatchLines false) ; 是否应该绘制线条
              )))
          (:then_1
            (goto _label_2 Reset)))
        (else
          (Utilities|FlowControl|Sequence ; 最后一位若为0则显示POI
            (:then_0
              (Utilities|FlowControl|DoOnce false :!label _label_2
                (:Completed
                  (if (Utilities|Name|Equal(Name) (Variables|/Game/Blueprints/GI_Nanjing.GI_Nanjing_C|GetCurrentLevelTag (Variables|Default|GetGameInstance)) (Utilities|Array|Get(acopy) (Variables|Default|GetTags))) ; 判断当前关卡名是否为自身所设置的Tag
                    (Development|SetHiddeninGame (Variables|Default|GetMaterialBiilboradComp) false false) ; Tag相同则显示
                    (Variables|Default|SetbShouldDrawBatchLines true) ; 是否应该绘制线条
                    (else
                      (Development|SetHiddeninGame (Variables|Default|GetMaterialBiilboradComp) true false) ; Tag不同则隐藏
                      (Variables|Default|SetbShouldDrawBatchLines false) ; 是否应该绘制线条
                      (Class|NdisplayPoiActor|ClearAllNdisplayPoiLines) ; 清除所有线条
                    )))))
            (:then_1
              (goto _label Reset))))))
    (:then_1
      (if (Variables|Default|GetbShouldDrawBatchLines)
        (Class|NdisplayPoiActor|DrawNdisplayPoiLine (Variables|Default|GetLinePositions)) ; 绘制线段
      ))))

(fn ConstructionScript
  (bind _returnvalue (Class|CriticalEditorSettings|GetCriticalEditorSettings))
  (bind _linepositions (Variables|Default|GetLinePositions))
  (bind _billboradsize (Variables|Default|GetBillboradSize))
  (bind _materialbiilboradcomp (Variables|Default|GetMaterialBiilboradComp))
  (bind _returnvalue_2 (Utilities|Array|LastIndex _linepositions))
  (bind _poiscalerate (Variables|/Script/CriticalSettings.CriticalEditorSettings|GetPoiScaleRate _returnvalue))
  (bind _output (Utilities|Array|Get(acopy) _linepositions _returnvalue_2))
  (bind (_leftlineoffset _rightlineoffset _uplineoffset _downlineoffset) (CallFunction|SelectPoiOffsetfromLastLinePoint _output))
  (Variables|Default|SetLineThickness (Variables|/Script/CriticalSettings.CriticalEditorSettings|GetPoiLineThickness (Class|CriticalEditorSettings|GetCriticalEditorSettings))) ; 设置线条粗细
  (Class|NdisplayPoiActor|DrawNdisplayPoiLine _linepositions) ; 画线
  (Transformation|SetWorldLocation (Variables|Default|GetMaterialBiilboradComp) (Utilities|Select :Index (Variables|PoiData|LineData|GetDirectionToOffsetPOI) :NewEnumerator0 _leftlineoffset :NewEnumerator1 _rightlineoffset :NewEnumerator2 _uplineoffset :NewEnumerator3 _downlineoffset) false false) ; 设置控件位置于线条末尾
  (Utilities|Array|SetArrayElem (Variables|/Script/Engine.MaterialBillboardComponent|GetElements _materialbiilboradcomp) 0 (Utilities|Struct|MakeMaterialSpriteElement "/NdisplayPOI/m_poi_Inst.m_poi_Inst" 0 false (* (.y _billboradsize) _poiscalerate) (* (.x _billboradsize) _poiscalerate)))
  (bind _returnvalue_3 (Rendering|Material|CreateDynamicMaterialInstance _materialbiilboradcomp 0 (Rendering|Material|GetMaterial _materialbiilboradcomp 0) "None" :!class /Script/Engine.PrimitiveComponent)) ; 设置POI所需材质实例
  (Rendering|Material|SetTextureParameterValue _returnvalue_3 "Image" (Variables|Default|GetPoiImage)) ; 通过材质实例设置POI图片
)

(fn SelectPoiOffsetfromLastLinePoint
  (params (LastPointLoc :type Vector))
  (bind (_x _y _z) (Math|Vector|BreakVector LastPointLoc))
  (bind (_x_2 _y_2 _z_2) (Math|Vector|BreakVector LastPointLoc))
  (bind _returnvalue (Class|CriticalEditorSettings|GetCriticalEditorSettings))
  (bind (_x_3 _y_3 _z_3) (Math|Vector|BreakVector LastPointLoc))
  (bind (_x_4 _y_4 _z_4) (Math|Vector|BreakVector LastPointLoc))
  (bind _billboradsize (Variables|Default|GetBillboradSize))
  (bind _poiscalerate (Variables|/Script/CriticalSettings.CriticalEditorSettings|GetPoiScaleRate _returnvalue))
  (bind _returnvalue_2 (* (.y _billboradsize) _poiscalerate))
  (bind _returnvalue_3 (* (.x _billboradsize) _poiscalerate))
  (return (Math|Vector|MakeVector (- _x_2 _returnvalue_3) _y_2 (+ _z_2 2.5e+02)) (Math|Vector|MakeVector (+ _x_3 _returnvalue_3) _y_3 (+ _z_3 2.5e+02)) (Math|Vector|MakeVector _x_4 (+ _y_4 _returnvalue_2) (+ _z_4 2.5e+02)) (Math|Vector|MakeVector _x (- _y _returnvalue_2) (+ _z 2.5e+02))))